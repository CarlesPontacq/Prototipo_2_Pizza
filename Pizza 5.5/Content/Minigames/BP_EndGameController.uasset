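; BP_EndGameController is a controller in the Minigames folder with click-to-move helpers and references to cooking minigame actors.
; Helpers trace under the cursor or finger, path to a location with a cursor effect, or steer the pawn toward it.
; GetMinigamesAndIngridients caches the first mill, grater, knife (BP_Regleta) and ingredient actors found in the level.
; BeginPlay and Tick are empty, and nothing here calls these functions.
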(event EventTick
  (params (DeltaSeconds :type Float%20%28single-precision%29)))

(event EventBeginPlay)

(fn ConstructionScript)

(fn Moveto
  (params (Location :type Vector))
  (AI|Navigation|SimpleMovetoLocation self Location)
  (Niagara|SpawnSystematLocation (Variables|Input|GetFXCursor) Location))

(fn Follow
  (params (Location :type Vector))
  (bind _returnvalue (Pawn|GetControlledPawn))
  (Pawn|Input|AddMovementInput _returnvalue (Math|Vector|GetUnitDirection(Vector) (Transformation|GetActorLocation _returnvalue) Location) 1.0 false))

(fn GetLocationUnderCursor
  (bind _hitresult (Game|Player|GetHitResultUnderCursorbyChannel "TraceTypeQuery1" true))
  (bind (_bblockinghit _binitialoverlap _time _distance _location _impactpoint _normal _impactnormal _physmat _hitactor) (Collision|BreakHitResult _hitresult))
  (return _bblockinghit _hitactor _location))

(fn GetLocationUnderFinger
  (bind _hitresult (Class|PlayerController|GetHitResultUnderFingerbyChannel "Touch1" "TraceTypeQuery1" false))
  (bind (_bblockinghit _binitialoverlap _time _distance _location) (Collision|BreakHitResult _hitresult))
  (return _bblockinghit _location))

(fn GetMinigamesandIngridients
  (bind _returnvalue (Actor|GetActorOfClass "/Game/Minigames/BP_Mill.BP_Mill_C"))
  (Variables|Default|SetMill _returnvalue)
  (bind _returnvalue_2 (Actor|GetActorOfClass "/Game/Minigames/BP_Grater.BP_Grater_C"))
  (Variables|Default|SetGrater _returnvalue_2)
  (bind _returnvalue_3 (Actor|GetActorOfClass "/Game/Minigames/BP_Regleta.BP_Regleta_C"))
  (Variables|Default|SetKnive _returnvalue_3)
  (bind _returnvalue_4 (Actor|GetActorOfClass "/Game/anim/BaconAnimado.BaconAnimado_C"))
  (Variables|Default|SetBaconAnimado _returnvalue_4)
  (bind _returnvalue_5 (Actor|GetActorOfClass "/Game/TopDown/Blueprints/BP_Oregano.BP_Oregano_C"))
  (Variables|Default|SetOregano _returnvalue_5)
  (bind _returnvalue_6 (Actor|GetActorOfClass "/Game/TopDown/Blueprints/BP_Cheese.BP_Cheese_C"))
  (Variables|Default|SetCheese _returnvalue_6)
  (bind _returnvalue_7 (Actor|GetActorOfClass "/Game/Minigames/QuesoRallado.QuesoRallado_C"))
  (Variables|Default|SetQuesoRallado _returnvalue_7))