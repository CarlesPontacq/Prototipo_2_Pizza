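; BP_Regleta is a minigame Blueprint with a Cursor that slides along the line between StartPoint and EndPoint.
; SetCursorPosition takes a hit location and moves the Cursor to its closest point on that line.
; The range check compares vector lengths from the world origin, so the Cursor moves only when the hit's length falls strictly between EndPoint's and StartPoint's.
; The event graph and construction script contain no logic.
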(event EventBeginPlay)

(event Collision|EventActorBeginOverlap
  (params (OtherActor :type Actor%20Object%20Reference)))

(event EventTick
  (params (DeltaSeconds :type Float%20%28single-precision%29)))

(fn ConstructionScript)

(fn SetCursorPosition
  (params (hitLocation :type Vector))
  (bind _returnvalue (Math|Vector|VectorLength hitLocation))
  (bind _endpoint (Variables|Default|GetendPoint))
  (bind _startpoint (Variables|Default|GetstartPoint))
  (bind _returnvalue_2 (Transformation|GetWorldLocation _startpoint))
  (bind _returnvalue_3 (Transformation|GetWorldLocation _endpoint))
  (if (< _returnvalue (Math|Vector|VectorLength _returnvalue_2))
    (if (> _returnvalue (Math|Vector|VectorLength _returnvalue_3))
      (Transformation|SetWorldLocation (Variables|Default|GetCursor) (Math|Vector|FindClosestPointonLine hitLocation _returnvalue_2 (- _returnvalue_2 _returnvalue_3)) false false))))