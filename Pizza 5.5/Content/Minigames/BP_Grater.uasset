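; Grater actor for a minigame that tracks how long an ingredient is being grated.
; BeginPlay stores Y-axis limits from two marker cubes, and a box overlap stores the touching BP_Ingredient, with no end-overlap clearing.
; Tick accumulates grate time while that ingredient moves, clearing the Grate flag past the finish time, though movement sets it again each frame.
; An uncalled helper derives and prints a max limit from grater scale.
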(event OnComponentBeginOverlap(Box)
  (params (OverlappedComponent :type Primitive%20Component%20Object%20Reference) (OtherActor :type Actor%20Object%20Reference) (OtherComp :type Primitive%20Component%20Object%20Reference) (OtherBodyIndex :type Integer) (bFromSweep :type Boolean) (SweepResult :type Hit%20Result%20Structure%20%28by%20ref%29))
  (bind _asbp_ingredient (Utilities|Casting|CastToBP_Ingredient OtherActor))
  (Variables|Default|SetIngredientOnGrater _asbp_ingredient))

(event EventBeginPlay
  ;[1 0 1] Set Grater Limits
  (Variables|Default|SetMaxLimit (.y (Transformation|GetWorldLocation (Variables|Default|GetMaxLimitCube))))
  (Variables|Default|SetMinLimit (.y (Transformation|GetWorldLocation (Variables|Default|GetMinLimitCube)))))

(event EventTick
  (params (DeltaSeconds :type Float%20%28single-precision%29))
  ;[1 0 1] Check if starts Grating
  (Utilities|FlowControl|Sequence
    (:then_0
      (if (Utilities|IsValid (Variables|Default|GetIngredientOnGrater))
        (if (Variables|/Game/TopDown/Blueprints/BP_Ingredient.BP_Ingredient_C|GetIsMoving (Variables|Default|GetIngredientOnGrater))
          (Variables|Default|SetGrate true)
          (else
            (Variables|Default|SetGrate false)))))
    (:then_1
      (if (Variables|Default|GetGrate)
        (bind _output_get (Variables|Default|SetgrateTime (+ (Variables|Default|GetgrateTime) DeltaSeconds)))
        (if (> _output_get (Variables|Default|GetfinishGrateTime))
          (Variables|Default|SetGrate false))))))

(fn ConstructionScript)

(fn CalculateLimitDistance
  (bind _grater (Variables|Default|GetGrater))
  (bind _returnvalue (Transformation|GetWorldLocation _grater))
  (bind _output_get (Variables|Default|SetMaxLimit (+ (.y _returnvalue) (* (.y _returnvalue) (/ (.y (Transformation|GetWorldScale (Variables|Default|GetGrater))) 2.0)))))
  (Development|PrintString (Utilities|String|ToString(Float) _output_get))
  (return _output_get))