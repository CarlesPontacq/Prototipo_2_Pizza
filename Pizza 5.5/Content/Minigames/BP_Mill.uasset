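; Coffee mill minigame actor in which the handle is rotated to grind through a set number of laps.
; SetMillRotation yaws the handle toward a supplied hit location until the minigame finishes.
; Tick checks handle yaw against milestone angles within a tolerance, counting a lap with a grinder sound once all are flagged.
; Start and finish flags drive a timeline slide of the animated mill mesh and its end animation, then set FinishedEndAnim.
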(event EventBeginPlay)

(event Collision|EventActorBeginOverlap
  (params (OtherActor :type Actor%20Object%20Reference)))

(event EventTick
  (params (DeltaSeconds :type Float%20%28single-precision%29))
  (bind _molinilloanim_3 (Variables|Default|GetMolinilloAnim_3))
  (Utilities|FlowControl|Sequence
    (:then_0
      ;[0.15 0.15 0.15 0.5] Drawers Anim
      (if (Variables|Default|GetstartMinigame)
        (bind _closedrawer (Timeline|BeginMiniGameAnim PlayFromStart)
          (:Update
            (Transformation|SetRelativeLocation (Variables|Default|GetMolinilloAnim_3) (Math|Vector|Lerp(Vector) (Variables|/Script/Engine.SceneComponent|GetRelativeLocation (Variables|Default|GetMolinilloAnim_3)) (Variables|/Script/Engine.SceneComponent|GetRelativeLocation (Variables|Default|GetEndPoint)) _closedrawer) false false))
          (:Finished
            (Variables|Default|SetstartMinigame false)))))
    (:then_1
      (if (Variables|Default|GetfinishMinigame)
        (Components|Timeline|PlayfromStart _molinilloanim_3)
        (Utilities|FlowControl|Delay (Media|MediaPlayer|GetDuration _molinilloanim_3))
        (Variables|Default|SetfinishMinigame false)
        (Variables|Default|SetfinishedEndAnim true)))
    (:then_2
      ;[0.15 0.15 0.15 0.5] Logic to detect full lap
      ;;[0 0.03967 0.849 0.5] Logic to detect if mill handle is in range of a milestone
      (for (_array_element _array_index) (Variables|Default|Getmilestones)
        (Variables|Default|Setindex _array_index)
        (Variables|Default|SetcurrentMilestoneToCheck _array_element)
        (Variables|Default|SetcurrentWorldRotationYaw (.yaw (Transformation|GetWorldRotation (Variables|Default|GetBaseSpin))))
        (Variables|Default|SetmaxRange (+ (Variables|Default|GetcurrentMilestoneToCheck) (Variables|Default|GetRange)))
        (Variables|Default|SetminRange (- (Variables|Default|GetcurrentMilestoneToCheck) (Variables|Default|GetRange)))
        ;;[0.1112 0.9146 0 0.5] Logic to set if the handle has been in range of a milestone in the lap
        (if (and (> (Variables|Default|GetcurrentWorldRotationYaw) (Variables|Default|GetminRange)) (< (Variables|Default|GetcurrentWorldRotationYaw) (Variables|Default|GetmaxRange)))
          (for (_array_element_2 _array_index_2) (Variables|Default|GetpassedMilestone)
            (if (== _array_index_2 (Variables|Default|Getindex))
              (if (not (Utilities|Array|Get(acopy) (Variables|Default|GetwasInRange) (Variables|Default|Getindex)))
                (if _array_element_2
                  (Utilities|Array|SetArrayElem (Variables|Default|GetpassedMilestone) (Variables|Default|Getindex) false)
                  (else
                    (Utilities|Array|SetArrayElem (Variables|Default|GetpassedMilestone) (Variables|Default|Getindex) true)
                    (Utilities|Array|SetArrayElem (Variables|Default|GetwasInRange) (Variables|Default|Getindex) true))))))
          (else
            (Utilities|Array|SetArrayElem (Variables|Default|GetwasInRange) (Variables|Default|Getindex) false))))
      ;;[0.7646 0.03348 0.5936 0.5] Logic to see if the full lap has been accomplished and if the minigame is finished
      (Variables|Default|SetfullLap true)
      (for _array_element_3 (Variables|Default|GetpassedMilestone)
        (if (not _array_element_3)
          (Variables|Default|SetfullLap false)))
      (if (Variables|Default|GetfullLap)
        (Development|PrintString (Utilities|String|ToString(Integer) (Variables|Default|GetcurrentLap)))
        (for (_ _array_index_3) (Variables|Default|GetpassedMilestone)
          (Utilities|Array|SetArrayElem (Variables|Default|GetpassedMilestone) _array_index_3 false))
        (bind _result (Math|Integer|IncrementInt (Variables|Default|GetcurrentLap))
          (:%20%20
            (Audio|PlaySound2D "/Game/TopDown/Sound/antique_manual_coffee_grinder-58439__mp3cut_net_.antique_manual_coffee_grinder-58439__mp3cut_net_" 1.0 1.0 0.0 0 0)
            (if (>= _result (Variables|Default|GetmaxLaps))
              (Variables|Default|SetfinishMinigame true))))))))

(fn ConstructionScript)

(fn SetMillRotation
  (params (HitLocation :type Vector))
  (if (not (Variables|Default|GetfinishMinigame))
    (Transformation|SetWorldRotation (Variables|Default|GetBaseSpin) (Math|Rotator|MakeRotator 0.0 0.0 (.yaw (Math|Rotator|FindLookatRotation (Transformation|GetWorldLocation (Variables|Default|GetBaseSpin)) HitLocation))) false false)))

(fn DetectFullRotation)